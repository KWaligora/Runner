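; Game mode for a runner game that tracks score and handles game over.
; It shows a score widget at start, then each tick while the player is alive sets Score to accumulated Points plus whole seconds of game time.
; GameOver stops scoring, shows a loss screen and runs a looping one-second timer that counts RestartTime down to zero, then restarts the level via console command.
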(event Custom|GameOver
  ;[1 1 1] Handle Game over
  (Variables|Default|SetPlayerAlive false)
  (bind _returnvalue (UserInterface|CreateWidget "/Game/Game/UI/LosseScreen.LosseScreen_C" (Game|GetPlayerController 0)))
  (UserInterface|Viewport|AddtoViewport _returnvalue 0)
  (Utilities|Time|SetTimerbyEvent (delegate Custom|RestartLevel) 1.0 true))

(event Custom|RestartLevel
  ;[1 1 1] Handle Game over
  (bind _result (Math|Integer|DecrementInt (Variables|Default|GetRestartTime))
    (:%20%20
      (bind _output_get (Variables|Default|SetRestartTime _result))
      (if (== _output_get 0)
        (Development|ExecuteConsoleCommand "RestartLevel" 0)))))

(event EventBeginPlay
  ;[1 1 1] Create Score UI
  (bind _returnvalue (UserInterface|CreateWidget "/Game/Game/UI/Score.Score_C" (Game|GetPlayerController 0)))
  (UserInterface|Viewport|AddtoViewport _returnvalue 0))

(event EventTick
  (params (DeltaSeconds :type Float%20%28single-precision%29))
  ;[1 1 1] Update Score if player is alive
  (if (Variables|Default|GetPlayerAlive)
    (CallFunction|UpdateScore)))

(fn ConstructionScript)

(fn IncreaseScore
  (params (points :type Integer))
  (Variables|Default|SetPoints (+ points (Variables|Default|GetPoints))))

(fn UpdateScore
  (Variables|Default|SetScore (+ (Variables|Default|GetPoints) (Math|Float|Truncate (Utilities|Time|GetGameTimeinSeconds)))))