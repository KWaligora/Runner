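; BP_Projectile is a Mage enemy projectile that kills the player on contact.
; Each tick it moves along negative world X by Speed scaled by delta time, offsetting from its Box component's world location rather than using a movement component.
; Overlapping a BP_Player calls OnDeath on that player without destroying the projectile, which removes itself after a short fixed lifetime.
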(event EventBeginPlay
  ;[1 1 1] LifeTime
  (Utilities|FlowControl|Delay 3.0)
  (Actor|DestroyActor))

(event EventTick
  (params (DeltaSeconds :type Float%20%28single-precision%29))
  (bind _box (Variables|Default|GetBox))
  (bind _returnvalue (Transformation|GetWorldLocation _box))
  ;[1 1 1] Move
  (Transformation|SetActorLocation (Math|Vector|MakeVector (- (.x _returnvalue) (* DeltaSeconds (Variables|Default|GetSpeed))) (.y _returnvalue) (.z _returnvalue)) false false))

(event Collision|EventActorBeginOverlap
  (params (OtherActor :type Actor%20Object%20Reference))
  ;[1 1 1] OnOverlap
  (bind _asbp_player (Utilities|Casting|CastToBP_Player OtherActor))
  (Class|PlayerCharacter|OnDeath _asbp_player))

(fn ConstructionScript)