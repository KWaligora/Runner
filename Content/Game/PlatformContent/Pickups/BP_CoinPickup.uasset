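; BP_CoinPickup is a coin pickup that adds points to the runner game's score when collected.
; On BeginPlay it casts the game mode to BP_RunnerGameMode and caches the reference.
; Its OnPickup override runs the parent pickup logic, plays a 2D retro coin sound and passes PointsReward to the game mode's IncreaseScore.
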(event EventOnPickup
  ;[1 1 1] OnPickup
  (|CallParentFunction)
  (Audio|PlaySound2D "/Game/Game/PlatformContent/Pickups/SoundEffects/retro-coin.retro-coin" 1.0 1.0 0.0 0 0)
  (Default|IncreaseScore (Variables|Default|GetGameMode) (Variables|Default|GetPointsReward)))

(event EventBeginPlay
  ;[1 1 1] Get GameMode
  (bind _asbp_runner_game_mode (Utilities|Casting|CastToBP_RunnerGameMode (Game|GetGameMode)))
  (Variables|Default|SetGameMode _asbp_runner_game_mode))

(fn ConstructionScript
  (|CallParentFunction))