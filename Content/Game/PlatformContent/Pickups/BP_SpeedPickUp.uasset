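; BP_SpeedPickUp is a pickup that temporarily scales the speed of the game's platforms.
; On BeginPlay it finds the BP_PlatformManager and caches its platform speed as the default.
; OnPickup runs the parent pickup logic, sets the manager's speed to the default times a boost multiplier, then restores the cached default after a delay of the effect duration.
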(event EventOnPickup
  (|CallParentFunction)
  (Class|PlatformManager|SetSpeed (Variables|Default|GetPlatformManager) (* (Variables|Default|GetDefaultSpeed) (Variables|Default|GetSpeedBoost)))
  (Utilities|FlowControl|Delay (Variables|Default|GetEffectDuration))
  (Class|PlatformManager|SetSpeed (Variables|Default|GetPlatformManager) (Variables|Default|GetDefaultSpeed)))

(event EventBeginPlay
  (bind _returnvalue (Actor|GetActorOfClass "/Game/Game/Platforms/BP_PlatformManager.BP_PlatformManager_C"))
  (Utilities|IsValid _returnvalue
    (:Is%20Valid
      (bind _output_get (Variables|Default|SetPlatformManager _returnvalue))
      (Variables|Default|SetDefaultSpeed (Variables|/Script/Runner.PlatformManager|GetPlatformSpeed _output_get)))))

(fn ConstructionScript
  (|CallParentFunction))