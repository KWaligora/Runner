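; BP_Player is the player character of a runner game, and its graph handles death.
; OnDeath is guarded by an IsDead flag so it only runs once.
; It plays a hurt sound, ragdolls the mesh through physics simulation, disables input and calls GameOver on BP_RunnerGameMode.
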(event EventOnDeath
  ;[1 1 1] OnDeath
  (if (not (Variables|Default|GetisDead))
    (Variables|Default|SetisDead true)
    (Audio|PlaySound2D "/Game/Game/Characters/SoundEffect/Ouch.Ouch" 1.0 1.0 0.0 0 0)
    (Physics|SetSimulatePhysics (Variables|Character|GetMesh) true)
    (Input|DisableInput (Game|GetPlayerController 0))
    (bind _asbp_runner_game_mode (Utilities|Casting|CastToBP_RunnerGameMode (Game|GetGameMode)))
    (Default|GameOver _asbp_runner_game_mode)))

(fn ConstructionScript)